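; ShapeHeroController is the player controller that handles hero respawning and the pause menu.
; On respawn it unpossesses, spawns a new ShapeHeroBP at the first PlayerStart found and possesses it, without destroying the old pawn.
; The Pause input toggles the UMG_MainMenu widget, using the stored widget reference as state to switch game pause, input mode and mouse cursor.
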(event `OnPlayerRespawn`
  (`self.UnPossess`)
  (bind _outactors (`GameplayStatics.GetAllActorsOfClass` "/Script/Engine.PlayerStart"))
  (bind _returnvalue (`|SpawnActorFromClass` "/Game/Blueprints/ShapeHeroBP.ShapeHeroBP_C" (`self.GetTransform` (`|GetArrayItem` _outactors)) "AlwaysSpawn" "OverrideRootScale" self null))
  (`self.Possess` _returnvalue))

(event `InputAction|Pause` :paused true
  (params (Key :type "Key Structure"))
  (bind _returnvalue (`GameplayStatics.GetPlayerController` 0))
  ;[1 1 1] Pause
  (:`Pressed`
    (`/Engine/EditorBlueprintResources/StandardMacros.IsValid` (`self.PauseUIRef`)
      (:`Is Valid`
        (`Widget.RemoveFromParent` (`self.PauseUIRef`))
        (set `self.PauseUIRef` null)
        (`WidgetBlueprintLibrary.SetInputMode_GameOnly` (`GameplayStatics.GetPlayerController` 0))
        (set `self.bShowMouseCursor` false)
        (`GameplayStatics.SetGamePaused` false))
      (:`Is Not Valid`
        (bind _returnvalue_2 (`|CreateWidget` "/Game/Widgets/UMG_MainMenu.UMG_MainMenu_C"))
        (bind _output_get (set `self.PauseUIRef` _returnvalue_2))
        (`UserWidget.AddToViewport` _output_get 0)
        (`WidgetBlueprintLibrary.SetInputMode_GameAndUIEx` _returnvalue null)
        (set `PlayerController.bShowMouseCursor` true _returnvalue)
        (`GameplayStatics.SetGamePaused` true)))))

(fn `UserConstructionScript`)